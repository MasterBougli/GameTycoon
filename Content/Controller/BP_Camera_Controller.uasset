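; Player controller that drives a BP_Camera_Pawn with movement, zoom and rotation input, and adds the WBP_Clock widget to the viewport.
; BeginPlay caches the pawn and its starting rotation for reset.
; Movement feeds the floating pawn movement along world axes regardless of camera yaw, while zoom steps the spring arm length within clamped limits.
; A gate passes mouse input to yaw and clamped pitch only while Rotation is held.
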(event `self.ReceiveBeginPlay`
  (`self.ReferenceCast`)
  (`self.SetDefault`)
  (`self.SetWidget`))

(event `InputAxis|MoveForward`
  (params (AxisValue :type "Float (single-precision)"))
  (`PawnMovementComponent.AddInputVector` (`/Game/Controller/BP_Camera_Pawn.FloatingPawnMovement` (`self.As BP Camera Pawn`)) (`KismetMathLibrary.MakeVector` AxisValue) false))

(event `InputAxis|MoveRight`
  (params (AxisValue :type "Float (single-precision)"))
  (`PawnMovementComponent.AddInputVector` (`/Game/Controller/BP_Camera_Pawn.FloatingPawnMovement` (`self.As BP Camera Pawn`)) (`KismetMathLibrary.MakeVector` 0.0 AxisValue) false))

(event `InputAction|ZoomOut`
  (params (Key :type "Key Structure"))
  (:`Pressed`
    (bind _output_get (set `self.ZoomInOut` -1.0))
    (`self.f_ZoomInOut` _output_get (`/Game/Controller/BP_Camera_Pawn.SpringArm` (`self.As BP Camera Pawn`)))))

(event `InputAction|ZoomIn`
  (params (Key :type "Key Structure"))
  (:`Pressed`
    (bind _output_get (set `self.ZoomInOut` 1.0))
    (`self.f_ZoomInOut` _output_get (`/Game/Controller/BP_Camera_Pawn.SpringArm` (`self.As BP Camera Pawn`)))))

(event `InputAction|ZoomReset`
  (params (Key :type "Key Structure"))
  (:`Pressed`
    (`self.f_ZoomReset` (`/Game/Controller/BP_Camera_Pawn.SpringArm` (`self.As BP Camera Pawn`)))))

(event `InputAction|Rotation`
  (params (Key :type "Key Structure"))
  (:`Pressed`
    (goto _label :!via `Open`))
  (:`Released`
    (goto _label :!via `Close`)))

(event `InputAction|Rotation`
  (params (Key :type "Key Structure"))
  (:`Pressed`
    (goto _label :!via `Open`))
  (:`Released`
    (goto _label :!via `Close`)))

(event `InputAxisKey|MouseX`
  (params (AxisValue :type "Float (single-precision)"))
  (`/Engine/EditorBlueprintResources/StandardMacros.Gate` true :!label _label
    (:`Exit`
      (`self.f_RotationSet` AxisValue (stale `InputAxisKey|MouseY` AxisValue)))))

(event `InputAxisKey|MouseY`
  (params (AxisValue :type "Float (single-precision)"))
  (goto _label))

(event `InputAction|RotationReset`
  (params (Key :type "Key Structure"))
  (:`Pressed`
    (`self.f_RotationReset`)))

(fn `f_RotationReset`
  (`self.K2_SetActorRotation` (`self.As BP Camera Pawn`) (`self.RotationDefault`) false))

(fn `f_RotationSet`
  (params (MouseX :type "Float (double-precision)") (MouseY :type "Float (double-precision)"))
  (bind _as_bp_camera_pawn (`self.As BP Camera Pawn`))
  (`self.K2_SetActorRotation` _as_bp_camera_pawn (`KismetMathLibrary.MakeRotator` (.roll (`self.K2_GetActorRotation` _as_bp_camera_pawn)) (`KismetMathLibrary.FClamp` (+ (.pitch (`self.K2_GetActorRotation` _as_bp_camera_pawn)) (* MouseY (`self.SpeedRotation`))) 10.0 70.0) (+ (.yaw (`self.K2_GetActorRotation` _as_bp_camera_pawn)) (* MouseX (`self.SpeedRotation`)))) false))

(fn `f_ZoomInOut`
  (params (Zoom :type "Float (double-precision)") (SpringArm :type "SpringArmComponent Object Reference"))
  (set `SpringArmComponent.TargetArmLength` (`KismetMathLibrary.FClamp` (+ (* Zoom (`self.SpeedZoom`)) (`SpringArmComponent.TargetArmLength` SpringArm)) 100.0 1500.0) SpringArm))

(fn `f_ZoomReset`
  (params (InputPin :type "SpringArmComponent Object Reference"))
  (set `SpringArmComponent.TargetArmLength` 1500.0 InputPin))

(fn `UserConstructionScript`)