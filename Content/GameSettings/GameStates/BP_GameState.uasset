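; Game state Blueprint that runs the in-game clock and calendar at an adjustable game speed.
; BeginPlay caches the camera controller, builds starting time and date from its variables, and applies the default speed.
; Each tick advances game time, derives hours, minutes and seconds, and rolls days into months and years using real month lengths.
; UpdateGameSpeed stores a multiplier, zeroes game time and calls GameSpeedControl.
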(event `self.ReceiveBeginPlay`
  (`|ExecutionSequence`
    (:`then_0`
      (`self.ReferenceCast`))
    (:`then_1`
      (`self.ReferenceTime`))
    (:`then_2`
      (`self.ReferenceClock`))))

(event `self.ReceiveTick`
  (params (DeltaSeconds :type "Float (single-precision)"))
  (set `self.NumberSecondPast` (+ (`self.NumberSecondPast`) 1.0))
  (bind (_gametime _daycount) (`/Game/Library/BPL_Function_Library.SetGameTime` DeltaSeconds (`self.Game Speed`) (`self.Game Time`)))
  (set `self.Game Time` _gametime)
  (set `self.Day Count` _daycount)
  (`self.SetClock`)
  (`self.SetCalendar`))

(event `/Game/Library/BPI_GameTime.UpdateGameSpeed`
  (params (SpeedMultiplier :type "Float (single-precision)"))
  (bind _output_get (set `self.SpeedMultiplier` SpeedMultiplier))
  (bind _output_get_2 (set `self.Game Time` 0.0))
  (`self.GameSpeedControl` _output_get_2))

(fn `SetCalendar`
  (bind _output_get (set `self.Days` (+ (`self.Days`) (`self.Day Count`))))
  (if (> _output_get (`KismetMathLibrary.DaysInMonth` (`self.Years`) (`self.Months`)))
    (set `self.Days` 1)
    (set `self.Months` (+ (`self.Months`) 1)))
  (if (> (`self.Months`) 12)
    (set `self.Months` 1)
    (set `self.Years` (+ (`self.Years`) 1)))
  (set `self.GameDate` (`|MakeArray` (`self.Days`) (`self.Months`) (`self.Years`))))

(fn `SetClock`
  (bind (_remainder _returnvalue) (`KismetMathLibrary.FMod` (* (`self.Game Time`) 3600.0) 60.0))
  (bind (_remainder_2 _returnvalue_2) (`KismetMathLibrary.FMod` (`KismetMathLibrary.Conv_IntToDouble` _returnvalue) 60.0))
  (set `self.Seconds` (`KismetMathLibrary.FFloor` _remainder))
  (set `self.Minutes` (`KismetMathLibrary.FFloor` _remainder_2))
  (set `self.Hours` (`KismetMathLibrary.FFloor` (`KismetMathLibrary.FMod` (`KismetMathLibrary.Conv_IntToDouble` _returnvalue_2) 24.0))))

(fn `UserConstructionScript`)