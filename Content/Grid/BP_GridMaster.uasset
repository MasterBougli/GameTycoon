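; BP_GridMaster is a grid actor that builds a tile layout in its Construction Script based on GridType.
; Nested loops over GridSize add child actor components: square tiles at fixed spacing, or hexagon tiles using SpacingX/SpacingY with alternate rows shifted by Offset.
; Octagon and triangle spawn functions are unfinished stubs that the Construction Script never calls.
; The event graph holds no active logic.
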(fn `UserConstructionScript`
  (switch `/Game/Grid/E_GridType` (`self.GridType`)
    (:`NewEnumerator1`
      (`self.SpawnSquare`))
    (:`NewEnumerator2`
      (`self.SpawnHexagon`))))